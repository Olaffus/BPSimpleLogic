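; Bullet projectile actor that deals its weapon's damage to the character it hits.
; On a Collision component hit, it casts the other actor to BP_Character, stores it and applies point damage, crediting the instigator's controller.
; The impact point is passed as the hit direction.
; A sequence node destroys the projectile after every hit, whether or not it struck a character.
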(event `self.Collision.OnComponentHit`
  (params (HitComponent :type "PrimitiveComponent Object Reference") (OtherActor :type "Actor Object Reference") (OtherComp :type "PrimitiveComponent Object Reference") (NormalImpulse :type "Vector Structure") (Hit :type "HitResult Structure (by ref)"))
  (`|ExecutionSequence`
    (:`then_0`
      (bind _asbp_character (cast `/Game/Blueprints/Character/BP_Character` OtherActor))
      (set `self.Character` _asbp_character)
      (`GameplayStatics.ApplyPointDamage` OtherActor (`/Game/Blueprints/Weapons/BP_Weapons.Damage` (`self.Weapon`)) (`.ImpactPoint` (`GameplayStatics.BreakHitResult` Hit)) Hit (`self.GetInstigatorController`) self))
    (:`then_1`
      (`self.K2_DestroyActor`))))

(fn `UserConstructionScript`
  (`parent.UserConstructionScript`))