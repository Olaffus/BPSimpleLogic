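; Automatic firearm weapon Blueprint, a child of a parent weapon class that supplies its use, add and construction behavior.
; The UseWeapon and AddWeapon events and the construction script only forward to the parent.
; Its Intarect override runs the parent interaction and, on success, sets itself as the interacting character's CurrentWeaponMain and returns true, otherwise false.
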(event `/Game/Blueprints/Weapons/BP_Weapons.UseWeapon`
  (`parent.UseWeapon`))

(event `/Game/Blueprints/Weapons/BP_Weapons.AddWeapon`
  (`parent.AddWeapon`))

(fn `Intarect`
  (params (Character :type "/Game/Blueprints/Character/BP_Character_Player Object Reference"))
  (returns (Success :type Boolean))
  (bind _success (`parent.Intarect` Character))
  (if _success
    (set `/Game/Blueprints/Character/BP_Character_Player.CurrentWeaponMain` self Character)
    (return true)
    (else
      (return false))))

(fn `UserConstructionScript`
  (`parent.UserConstructionScript`))