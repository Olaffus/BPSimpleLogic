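; Weapon Blueprint that fires a projectile from the weapon toward the point the player's camera is aimed at.
; UseWeapon runs the parent logic, then spawns the projectile ahead of the skeletal mesh along camera forward, passing weapon and instigator.
; A Visibility line trace from the camera finds the aim target, falling back to the trace end on a miss, so shots converge on screen center.
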(event `self.UseWeapon`
  (`parent.UseWeapon`)
  (`self.ProjectileSpawn`))

(fn `LineTrace_FindEndTarget`
  (returns (TraceEnd :type "Vector Structure"))
  (bind _asbp_character_player (cast `/Game/Blueprints/Character/BP_Character_Player` (`self.UseCharacter`)))
  (bind _camera (`/Game/Blueprints/Character/BP_Character_Player.Camera` _asbp_character_player))
  (bind _returnvalue (`SceneComponent.K2_GetComponentLocation` _camera))
  (bind _returnvalue_2 (+ _returnvalue (* (`SceneComponent.GetForwardVector` _camera) 10000.0)))
  (bind (_outhit _returnvalue_3) (`KismetSystemLibrary.LineTraceSingle` _returnvalue _returnvalue_2 "TraceTypeQuery1"))
  (if _returnvalue_3
    (return (`.ImpactPoint` (`GameplayStatics.BreakHitResult` _outhit)))
    (else
      (return _returnvalue_2))))

(fn `ProjectileSpawn`
  (bind _asbp_character_player (cast `/Game/Blueprints/Character/BP_Character_Player` (`self.UseCharacter`)))
  (bind _returnvalue (+ (`SceneComponent.K2_GetComponentLocation` (`self.SkeletalMesh`)) (* (`SceneComponent.GetForwardVector` (`/Game/Blueprints/Character/BP_Character_Player.Camera` _asbp_character_player)) 100.0)))
  (`|SpawnActorFromClass` (`self.Projectile`) (`KismetMathLibrary.MakeTransform` _returnvalue (`KismetMathLibrary.FindLookAtRotation` _returnvalue (`self.LineTrace_FindEndTarget`))) "AlwaysSpawn" "OverrideRootScale" self self (`PawnMovementComponent.GetPawnOwner` (`Character.CharacterMovement` (`self.UseCharacter`)))))

(fn `UserConstructionScript`
  (`parent.UserConstructionScript`))