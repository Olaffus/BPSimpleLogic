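; BP_HealthComponent is a player health component that tracks Health and triggers the owning character's death.
; On BeginPlay it casts its owner to BP_Character and stores that reference.
; ChangeHealth subtracts the given value, clamps only at zero, and calls Death when Health is depleted.
; Death hands off to the character's Dead function, passing the character's own IsDeadHead value.
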(event `self.ReceiveBeginPlay`
  ;[1 1 1] Получаем ссылку на владельца компонента
  (bind _asbp_character (cast `/Game/Blueprints/Character/BP_Character` (`self.GetOwner`)))
  (set `self.Character` _asbp_character))

(fn `ChangeHealth`
  (params (Value :type "Float (double-precision)"))
  (bind _output_get (set `self.Health` (- (`self.Health`) Value)))
  (if (<= _output_get 0.0)
    (set `self.Health` 0.0)
    (`self.Death`)))

(fn `Death`
  (bind _character (`self.Character`))
  (`/Game/Blueprints/Character/BP_Character.Dead` _character (`/Game/Blueprints/Character/BP_Character.isDead_Head` _character)))