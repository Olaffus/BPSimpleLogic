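; Aggressive NPC character that spots the player, builds up alarm and opens fire.
; Pawn sensing starts a looping WaitAlarmed timer that registers it with the player, line-traces for sight, turns toward them and raises an alarm counter, shooting bullets past a threshold.
; When sight breaks, it runs to the last seen location via its AI controller, then LostTarget deregisters it and resumes roaming.
; Tick clears timer and target on death.
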(event `self.ReceiveBeginPlay`
  ;[1 1 1] Comment
  (`parent.ReceiveBeginPlay`))

(event `self.PawnSensing.OnSeePawn`
  (params (Pawn :type "Pawn Object Reference"))
  ;[1 1 1] OnSee
  (bind _asbp_character_player (cast `/Game/Blueprints/Character/BP_Character_Player` Pawn))
  (set `self.Target` Pawn)
  (if (== (`GameplayStatics.GetObjectClass` _asbp_character_player) "/Game/Blueprints/Character/BP_Character_Player.BP_Character_Player_C")
    (bind _returnvalue (`KismetSystemLibrary.K2_SetTimer` null "WaitAlarmed" 0.1 true))
    (set `self.TimerWaitAlarmed` _returnvalue)))

(event `self.ReceiveTick`
  (params (DeltaSeconds :type "Float (single-precision)"))
  ;[1 1 1] EventTick
  ;;[1 1 1] IsDead
  (if (not (`self.isDead`))
    (`self.Target`
      (:`then`)
      (:`else`))
    (else
      (`KismetSystemLibrary.K2_ClearAndInvalidateTimerHandle` (`self.TimerWaitAlarmed`))
      (set `self.Target` null))))

(fn `Alarmed`)

(fn `Attack_SpawnProjectile`
  (`|SpawnActorFromClass` "/Game/Blueprints/Weapons/Projectile/BP_Projectile_Bullets.BP_Projectile_Bullets_C" (`KismetMathLibrary.MakeTransform` (+ (`self.K2_GetActorLocation` self) (* (`self.GetActorForwardVector` self) 100.0)) (`self.K2_GetActorRotation`) (1.0 1.0 1.0)) "Undefined" "OverrideRootScale" self (`self.WeaponFireAutomat`) self))

(fn `LostTarget`
  (set `self.isRunning` false)
  (`KismetArrayLibrary.Array_RemoveItem` (`/Game/Blueprints/Character/BP_Character_Player.ListEnemyAlarmed` (cast `/Game/Blueprints/Character/BP_Character_Player` (`self.Target`) :!pure true)) self)
  (`KismetSystemLibrary.K2_ClearAndInvalidateTimerHandle` (`self.TimerWaitAlarmed`))
  (set `self.Target` null)
  (`/Game/Blueprints/Character/NPC/Components/MainComponents.Start` (`/Game/Blueprints/Character/NPC/BP_AIControllerNPC.BP_RoamingComponents` (cast `/Game/Blueprints/Character/NPC/Agressive/BP_AIControllerNPC_Agressive` (`self.GetController`) :!pure true))))

(fn `Rotate`
  (bind (_returnvalue_roll _returnvalue_pitch _returnvalue_yaw) (`KismetMathLibrary.BreakRotator` (`KismetMathLibrary.Conv_VectorToRotator` (`KismetMathLibrary.GetDirectionUnitVector` (`self.K2_GetActorLocation`) (`self.K2_GetActorLocation` (`self.Target`))))))
  (`self.K2_SetActorRotation` (`KismetMathLibrary.RInterpTo_Constant` (`self.K2_GetActorRotation`) (`KismetMathLibrary.MakeRotator` 0.0 0.0 _returnvalue_yaw) 0.05 500.0)))

(fn `UserConstructionScript`
  (`parent.UserConstructionScript`))

(fn `WaitAlarmed`
  (bind _target (`self.Target`))
  (bind _timewaitalarmed (`self.TimeWaitAlarmed`))
  (bind _asbp_character_player (cast `/Game/Blueprints/Character/BP_Character_Player` (`self.Target`) :!pure true))
  (if (not (`/Game/Blueprints/Character/BP_Character.isDead` (cast `/Game/Blueprints/Character/BP_Character` (`self.Target`) :!pure true)))
    (if (== (`KismetArrayLibrary.Array_Find` (`/Game/Blueprints/Character/BP_Character_Player.ListEnemyAlarmed` (cast `/Game/Blueprints/Character/BP_Character_Player` (`self.Target`) :!pure true)) self) -1)
      (`KismetArrayLibrary.Array_Add` (`/Game/Blueprints/Character/BP_Character_Player.ListEnemyAlarmed` (cast `/Game/Blueprints/Character/BP_Character_Player` (`self.Target`) :!pure true)) self))
    (bind _outhit (`KismetSystemLibrary.LineTraceSingle` (`self.K2_GetActorLocation` self) (`self.K2_GetActorLocation` (`self.Target`)) "TraceTypeQuery1"))
    (if (== (`.HitActor` (`GameplayStatics.BreakHitResult` _outhit)) (`self.Target`))
      (`self.Rotate`)
      (`/Engine/EditorBlueprintResources/StandardMacros.IncrementFloat` (`self.TimeWaitAlarmed`)
        (:`  `
          (if (> (`self.TimeWaitAlarmed`) 10.0)
            (`self.Attack_SpawnProjectile`)
            (set `self.L_oldPlaceTarget_` (`self.K2_GetActorLocation` _target) :!label _label)
            (`/Game/Blueprints/Character/NPC/Agressive/BP_AIControllerNPC_Agressive.Stop` (cast `/Game/Blueprints/Character/NPC/Agressive/BP_AIControllerNPC_Agressive` (`self.GetController`) :!pure true))
            (set `self.isTargetRifles` true)
            (if (< (`/Game/Blueprints/Character/BP_Character_Player.ValueAlarmed` _asbp_character_player) _timewaitalarmed)
              (set `/Game/Blueprints/Character/BP_Character_Player.ValueAlarmed` _timewaitalarmed _asbp_character_player))
            (else
              (bind _outhit_2 (`KismetSystemLibrary.LineTraceSingle` (`self.K2_GetActorLocation` self) (`self.K2_GetActorLocation` (`self.Target`)) "TraceTypeQuery1"))
              (if (== (`.HitActor` (`GameplayStatics.BreakHitResult` _outhit_2)) _target)
                (goto _label)
                (else
                  (set `self.isTargetRifles` false :!label _label_2)
                  (set `self.isRunning` true)
                  (bind _returnvalue (`AIController.MoveToLocation` (cast `/Game/Blueprints/Character/NPC/Agressive/BP_AIControllerNPC_Agressive` (`self.GetController`) :!pure true) (`self.L_oldPlaceTarget_`) 50.0 true true true true null true))
                  (switch `EPathFollowingRequestResult` _returnvalue
                    (:`RequestSuccessful`
                      (`KismetSystemLibrary.K2_SetTimer` null "LostTarget" 2.0)))))))))
      (else
        (goto _label_2)))
    (else
      (set `self.isTargetRifles` false)
      (set `self.isRunning` false))))