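; NPC component that makes a character wander between random navigable points near its current position while roaming is active.
; Start enables walking and picks a target; Stop halts movement and clears both timers.
; A looping timer reissues the AI MoveToLocation every half second, using the "Already at Goal" result to detect arrival instead of a completion callback.
; On arrival, a delay timer pauses the NPC before choosing the next point.
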(event `self.Start`
  (`parent.Start`)
  (set `self.isRoaming` true)
  (set `/Game/Blueprints/Character/BP_Character.isWalking` true (`self.NPC_MC`))
  (`self.GoToNewTarget`))

(event `self.Stop`
  (`parent.Stop`)
  (`MovementComponent.StopMovementImmediately` (`Character.CharacterMovement` (`self.NPC_MC`)))
  (`KismetSystemLibrary.K2_ClearAndInvalidateTimerHandle` (`self.DelayTimer`))
  (`KismetSystemLibrary.K2_ClearAndInvalidateTimerHandle` (`self.MoveToTimer`))
  (set `self.isRoaming` false))

(fn `FindRoamTarget`
  (returns (TargetLocation :type "Vector Structure"))
  (bind _outactors (`GameplayStatics.GetAllActorsOfClass` "/Script/Engine.NavigationData"))
  (return (`NavigationSystem.K2_GetRandomLocationInNavigableRadius` (`|GetArrayItem` _outactors) (`Actor.K2_GetActorLocation` (`self.NPC_MC`)) (`self.FindTargetRadius`))))

(fn `GoToNewTarget`
  (bind _targetlocation (`self.FindRoamTarget`))
  (set `self.TargetLocation` _targetlocation)
  (bind _returnvalue (`KismetSystemLibrary.K2_SetTimer` null "GoToTarget" 0.5 true))
  (set `self.MoveToTimer` _returnvalue)
  (set `self.isWaiting` false)
  (set `self.isMoving` true))

(fn `GoToTarget`
  (bind _returnvalue (`AIController.MoveToLocation` (`self.NPCController_MC`) (`self.TargetLocation`) 50.0 true true false true null true))
  (switch `EPathFollowingRequestResult` _returnvalue
    (:`AlreadyAtGoal`
      (`self.TargetReached`))))

(fn `TargetReached`
  (`KismetSystemLibrary.K2_ClearAndInvalidateTimerHandle` (`self.MoveToTimer`))
  (bind _returnvalue (`KismetSystemLibrary.K2_SetTimer` null "GoToNewTarget" (`self.StopDelay`)))
  (set `self.DelayTimer` _returnvalue)
  (set `self.isWaiting` true)
  (set `self.isMoving` false))