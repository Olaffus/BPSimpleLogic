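; BP_Character is a character Blueprint handling movement speed, hit-location damage and death.
; Head and capsule hit events flag where it was struck, and AnyDamage waits a tick before passing doubled head or halved body damage to BPHealthComponent.
; Looping timers poll walk, run and sprint flags to set MaxWalkSpeed.
; Dead records the hit zone, disables movement and capsule collision, then ragdolls the mesh after a delay.
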(event `self.CapsuleComponent.OnComponentHit`
  (params (HitComponent :type "PrimitiveComponent Object Reference") (OtherActor :type "Actor Object Reference") (OtherComp :type "PrimitiveComponent Object Reference") (NormalImpulse :type "Vector Structure") (Hit :type "HitResult Structure (by ref)"))
  ;[1 0.07485 0.1946] AnyDamage
  (set `self.isDead_Head` false)
  (set `self.isDead_Body` true))

(event `self.Head.OnComponentHit`
  (params (HitComponent :type "PrimitiveComponent Object Reference") (OtherActor :type "Actor Object Reference") (OtherComp :type "PrimitiveComponent Object Reference") (NormalImpulse :type "Vector Structure") (Hit :type "HitResult Structure (by ref)"))
  ;[1 0.07485 0.1946] AnyDamage
  (set `self.isDead_Head` true)
  (set `self.isDead_Body` false))

(event `self.ReceiveAnyDamage`
  (params (Damage :type "Float (single-precision)") (DamageType :type "DamageType Object Reference") (InstigatedBy :type "Controller Object Reference") (DamageCauser :type "Actor Object Reference"))
  ;[1 0.07485 0.1946] AnyDamage
  (`KismetSystemLibrary.Delay` 0.001)
  (`/Game/Blueprints/Components/Player/BP_HealthComponent.ChangeHealth` (`self.BP_HealthComponent`) (`KismetMathLibrary.SelectFloat` (* Damage 2.0) (/ Damage 2.0) (`self.isDead_Head`))))

(event `self.ReceiveBeginPlay`
  (set `self.isWalking` true)
  (set `self.isRunning` false)
  (set `self.isSprint` false)
  ;[1 1 1] SetWaking
  (`KismetSystemLibrary.K2_SetTimer` null "SetWaking" 0.1 true)
  ;[1 1 1] SetTimerRunning
  (`KismetSystemLibrary.K2_SetTimer` null "SetRunning" 0.1 true)
  ;[1 1 1] SetTimerSprint
  (`KismetSystemLibrary.K2_SetTimer` null "SetSprint" 0.1 true))

(fn `Dead`
  (params (isDead_Head :type Boolean))
  (set `self.isDead` true)
  (if isDead_Head
    (set `self.isDead_Head` true)
    (set `self.isDead_Body` false)
    (else
      (set `self.isDead_Body` true)
      (set `self.isDead_Head` false)))
  (`CharacterMovementComponent.DisableMovement` (`self.CharacterMovement`))
  (`PrimitiveComponent.SetCollisionEnabled` (`self.CapsuleComponent`) "NoCollision")
  (`PrimitiveComponent.SetCollisionEnabled` (`self.Mesh`) "QueryAndPhysics")
  (`KismetSystemLibrary.K2_SetTimer` null "SimulatePhysicsSet" 1.5))

(fn `SetRunning`
  (if (and (`self.isRunning`) (== (`self.isSprint`) false))
    (set `CharacterMovementComponent.MaxWalkSpeed` (`self.RunValue`) (`self.CharacterMovement`))))

(fn `SetSprint`
  (if (`self.isSprint`)
    (set `CharacterMovementComponent.MaxWalkSpeed` (`self.SprintValue`) (`self.CharacterMovement`))
    (set `self.isWalking` false)
    (set `self.isRunning` false)))

(fn `SetWaking`
  (if (and (== (`self.isRunning`) false) (== (`self.isSprint`) false))
    (set `CharacterMovementComponent.MaxWalkSpeed` (`self.WalkValue`) (`self.CharacterMovement`))))

(fn `SimulatePhysicsSet`
  (`PrimitiveComponent.SetSimulatePhysics` (`self.Mesh`) true))

(fn `UserConstructionScript`)