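; Touch-controlled pawn that either launches a Ball or rotates the camera, depending on where a press lands.
; Pressing the ball sets its Hold flag and shows the Cursor; releasing hides the Cursor and calls BallLaunch if the ball was held.
; Pressing elsewhere records the start X and yaw and opens a Gate, letting Tick turn the actor's yaw with horizontal drag until release.
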(event `self.ReceiveTick`
  (params (DeltaSeconds :type "Float (single-precision)"))
  (`/Engine/EditorBlueprintResources/StandardMacros.Gate` true :!label _label
    (:`Exit`
      (`self.moveCamera`))))

(event `InputTouch`
  (params (Location :type "Vector Structure") (FingerIndex :type "ETouchIndex Enum"))
  (bind _returnvalue (!= (`self.touchBall`) (`self.Ball`)))
  (:`Pressed`
    (`|ExecutionSequence`
      (:`then_0`
        (if _returnvalue
          (`self.initCameraRot` Location
            (:`Open`
              (goto _label :!via `Open`)))
          (else
            (`self.ballMove` :!label _label_2))))
      (:`then_1`
        (if (not _returnvalue)
          (`SceneComponent.SetHiddenInGame` (`self.cursor`) false false)))))
  (:`Released`
    (`SceneComponent.SetHiddenInGame` (`self.cursor`) true false)
    (`|ExecutionSequence`
      (:`then_0`
        (goto _label_2 :!via `Unpressed`))
      (:`then_1`
        (goto _label :!via `Close`)))))

(fn `UserConstructionScript`)