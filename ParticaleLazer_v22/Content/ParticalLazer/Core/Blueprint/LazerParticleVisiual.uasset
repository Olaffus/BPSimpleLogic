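; Laser beam visual actor that stretches a particle system between a start point and an end point.
; On BeginPlay it spawns two collision-disabled BP_Point actors, then adds a particle component bound to them through Actor_Source and Actor_Target instance parameters.
; Tick moves both points to StartLocation and EndLocation every frame.
; SetLocation moves the points directly without updating those variables, so Tick overrides it.
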(event `self.ReceiveBeginPlay`
  (`|ExecutionSequence`
    (:`then_0`
      (bind _returnvalue (`|SpawnActorFromClass` "/Game/ParticalLazer/Core/Blueprint/BP_Point.BP_Point_C" (`KismetMathLibrary.MakeTransform` (`self.StartLocation`)) "Undefined" "OverrideRootScale" null null))
      (bind _output_get (set `self.StartPoint` _returnvalue))
      (`self.SetActorEnableCollision` _output_get false))
    (:`then_1`
      (bind _returnvalue_2 (`|SpawnActorFromClass` "/Game/ParticalLazer/Core/Blueprint/BP_Point.BP_Point_C" (`KismetMathLibrary.MakeTransform` (`self.EndLocation`)) "Undefined" "OverrideRootScale" null null))
      (bind _output_get_2 (set `self.EndPoint` _returnvalue_2))
      (`self.SetActorEnableCollision` _output_get_2 false))
    (:`then_2`
      (bind _returnvalue_3 (`AddComponent|NODE_AddParticleSystemComponent-0`))
      (bind _output_get_3 (set `self.Particle` _returnvalue_3))
      (set `ParticleSystemComponent.InstanceParameters` (`|MakeArray` (make `ParticleSysParam` "Actor_Source" "PSPT_Actor" 0.0 0.0 (0.0 0.0 0.0) (0.0 0.0 0.0) (struct) (`self.StartPoint`)) (make `ParticleSysParam` "Actor_Target" "PSPT_Actor" 0.0 0.0 (0.0 0.0 0.0) (0.0 0.0 0.0) (struct) (`self.EndPoint`))) _output_get_3))))

(event `self.ReceiveTick`
  (params (DeltaSeconds :type "Float (single-precision)"))
  (`self.K2_SetActorLocation` (`self.StartPoint`) (`self.StartLocation`) false false)
  (`self.K2_SetActorLocation` (`self.EndPoint`) (`self.EndLocation`) false false))

(fn `SetLocation`
  (params (Start :type "Vector Structure") (End :type "Vector Structure"))
  (`self.K2_SetActorLocation` (`self.StartPoint`) Start false false)
  (`self.K2_SetActorLocation` (`self.EndPoint`) End false false))

(fn `UserConstructionScript`)