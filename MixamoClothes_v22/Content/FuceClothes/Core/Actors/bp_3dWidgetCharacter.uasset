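; Preview character actor, apparently for a 3D widget, that shows the player's clothing and can be turned with the mouse.
; Click start and end events toggle rotation, and mouse moves yaw the skeletal mesh by the inverted horizontal delta.
; The Cloth component follows the body's skeleton through master pose.
; Update copies the clothing mesh from the referenced ThirdPersonCharacter onto Cloth.
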(event `ClickedStart`
  (params (MouseLocation :type "Vector2D Structure"))
  ;[1 1 1] Вращение пресонажа по z
  (set `self.startLocation` MouseLocation)
  (set `self.isRotation?` true))

(event `ClickedEnd`
  ;[1 1 1] Вращение пресонажа по z
  (set `self.isRotation?` false))

(event `MouseMove`
  (params (MouseLocation :type "Vector2D Structure") (startLocation :type "Vector2D Structure"))
  (bind _returnvalue_x (`KismetMathLibrary.BreakVector2D` (- MouseLocation (`self.startLocation`))))
  ;[1 1 1] Вращение пресонажа по z
  (if (`self.isRotation?`)
    (`SceneComponent.K2_AddWorldRotation` (`self.SkeletalMesh`) (`KismetMathLibrary.MakeRotator` 0.0 0.0 (* _returnvalue_x -1.0)) false false)
    (set `self.startLocation` MouseLocation)))

(fn `-Update`
  (`SkinnedMeshComponent.SetSkinnedAssetAndUpdate` (`self.Cloth`) (`SkinnedMeshComponent.SkeletalMesh` (`/Game/FuceClothes/Core/Characters/ThirdPersonCharacter.ClothingMesh` (`self.ThirdPersonCharacter`))) true))

(fn `UserConstructionScript`
  (`SkinnedMeshComponent.SetLeaderPoseComponent` (`self.Cloth`) (`self.SkeletalMesh`) false))